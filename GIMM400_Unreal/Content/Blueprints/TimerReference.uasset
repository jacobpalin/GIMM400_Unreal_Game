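; Countdown match timer Blueprint that ends the game in what appears to be a hider win when time runs out.
; Tick feeds a one-second Delay, so Seconds drops about once per second and rolls over into Minutes.
; At zero it creates a widget, adds it to the viewport, shows the mouse cursor and pauses the game.
; The graph cites a Matt Aspland YouTube tutorial.
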(event `self.ReceiveTick`
  (params (DeltaSeconds :type "Float (single-precision)"))
  ;[1 1 1] video: https://www.youtube.com/watch?v=nHK97x6ILYo&ab_channel=MattAspland
  (`KismetSystemLibrary.Delay` 1.0)
  (if (== (`self.Seconds`) 0)
    (if (== (`self.Minutes`) 0)
      (bind _returnvalue (`|CreateWidget` "/Game/Blueprints/UI/HiderWin.HiderWin_C"))
      (`UserWidget.AddToViewport` _returnvalue 0)
      (set `PlayerController.bShowMouseCursor` true (`GameplayStatics.GetPlayerController` 0))
      (`GameplayStatics.SetGamePaused` true)
      (else
        (set `self.Seconds` 59)
        (set `self.Minutes` (- (`self.Minutes`) 1))))
    (else
      (set `self.Seconds` (- (`self.Seconds`) 1)))))

(fn `UserConstructionScript`)