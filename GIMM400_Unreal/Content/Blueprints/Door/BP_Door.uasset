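; BP_Door is a swinging door that the third-person character opens and closes with the E key.
; Its box trigger enables input, stores the player reference and shows an E prompt widget, then disables input and attempts to remove the prompt on exit.
; A dot product picks the swing direction from the player's side.
; The OpenDoor timeline interpolates yaw, auto-reverses after a delay and marks the door closed when the reverse finishes.
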(event `Key|E`
  (params (Key :type "Key Structure"))
  (bind _defaultsceneroot (`self.DefaultSceneRoot`))
  ;[1 1 1] door video: https://www.youtube.com/watch?v=hZHj5CtonQA&ab_channel=CobbDev
  (:`Pressed`
    (if (`self.IsDoorClosed`)
      (set `self.IsDoorClosed` false)
      (set `self.DotProduct` (`KismetMathLibrary.Dot_VectorVector` (`KismetMathLibrary.Normal` (- (`SceneComponent.K2_GetComponentLocation` _defaultsceneroot) (`self.K2_GetActorLocation` (`self.PlayerRef`)))) (`SceneComponent.GetForwardVector` _defaultsceneroot)))
      (bind (_direction _alpha) (`Timeline|Open Door` :!label _label)
        (:`Update`
          (`SceneComponent.K2_SetRelativeRotation` (`self.Door`) (`KismetMathLibrary.MakeRotator` 0.0 0.0 (`KismetMathLibrary.Lerp` 0.0 (`KismetMathLibrary.SelectFloat` 90.0 -90.0 (>= (`self.DotProduct`) 0.0)) _alpha)) false false)
          ;[1 1 1] closes after delay (delete because this kinda sucks
          (if (not (`self.IsDoorClosed`))
            (`KismetSystemLibrary.Delay` 5.0)
            (goto _label :!via `Reverse`)))
        (:`Finished`
          (switch `ETimelineDirection` _direction
            (:`Backward`
              (set `self.IsDoorClosed` true)))))
      (else
        (goto _label :!via `Reverse`)))))

(event `self.Box.OnComponentBeginOverlap`
  (params (OverlappedComponent :type "PrimitiveComponent Object Reference") (OtherActor :type "Actor Object Reference") (OtherComp :type "PrimitiveComponent Object Reference") (OtherBodyIndex :type Integer) (bFromSweep :type Boolean) (SweepResult :type "HitResult Structure (by ref)"))
  (bind _returnvalue (`GameplayStatics.GetPlayerController` 0))
  (bind _asbp_third_person_character (cast `/Game/ThirdPerson/Blueprints/BP_ThirdPersonCharacter` OtherActor))
  (`self.EnableInput` _returnvalue)
  (bind _returnvalue_2 (`|CreateWidget` "/Game/Blueprints/E_Text/E_Widget.E_Widget_C" _returnvalue))
  (`UserWidget.AddToViewport` _returnvalue_2 0)
  (set `self.PlayerRef` _asbp_third_person_character))

(event `self.Box.OnComponentEndOverlap`
  (params (OverlappedComponent :type "PrimitiveComponent Object Reference") (OtherActor :type "Actor Object Reference") (OtherComp :type "PrimitiveComponent Object Reference") (OtherBodyIndex :type Integer))
  (bind _returnvalue (`GameplayStatics.GetPlayerController` 0))
  (cast `/Game/ThirdPerson/Blueprints/BP_ThirdPersonCharacter` OtherActor)
  (`self.DisableInput` _returnvalue)
  (`|CreateWidget` "/Game/Blueprints/E_Text/E_Widget.E_Widget_C" _returnvalue)
  (`Widget.RemoveFromParent` (stale `self.Box.OnComponentBeginOverlap` _returnvalue_2)))

(fn `UserConstructionScript`)